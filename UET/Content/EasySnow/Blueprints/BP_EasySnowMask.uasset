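; BP_EasySnowMask is a placeable box actor that defines a custom snow mask area for EasySnow materials.
; It writes the box's world location and scale, plus edge falloff and breakup tiling and contrast, into the MP_WF_WorldData material parameter collection.
; The same writes run in the Construction Script for editor preview and again on BeginPlay.
; Because the collection is global, each instance overwrites the same parameters.
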(event EventBeginPlay
  (bind _box (Variables|Default|GetBox))
  (Rendering|Material|SetVectorParameterValue "/Game/EasySnow/System/MP_WF_WorldData.MP_WF_WorldData" "Location" (Math|Conversions|ToLinearColor(Vector) (Transformation|GetWorldLocation _box)) :!class /Script/Engine.KismetMaterialLibrary)
  (Rendering|Material|SetVectorParameterValue "/Game/EasySnow/System/MP_WF_WorldData.MP_WF_WorldData" "Scale" (Math|Conversions|ToLinearColor(Vector) (Transformation|GetWorldScale _box)) :!class /Script/Engine.KismetMaterialLibrary)
  (Rendering|Material|SetScalarParameterValue "/Game/EasySnow/System/MP_WF_WorldData.MP_WF_WorldData" "Custom Snow Mask Edge Falloff" (Variables|Default|GetcustomSnowMaskEdgeFalloff) :!class /Script/Engine.KismetMaterialLibrary)
  (Rendering|Material|SetScalarParameterValue "/Game/EasySnow/System/MP_WF_WorldData.MP_WF_WorldData" "Custom Snow Mask Breakup Tiling" (Variables|Default|GetcustomSnowMaskBreakupTiling) :!class /Script/Engine.KismetMaterialLibrary)
  (Rendering|Material|SetScalarParameterValue "/Game/EasySnow/System/MP_WF_WorldData.MP_WF_WorldData" "Custom Snow Mask Breakup Contrast" (Variables|Default|GetcustomSnowMaskBreakupContrast) :!class /Script/Engine.KismetMaterialLibrary))

(event Collision|EventActorBeginOverlap
  (params (OtherActor :type Actor%20Object%20Reference)))

(event EventTick
  (params (DeltaSeconds :type Float%20%28single-precision%29)))

(fn ConstructionScript
  (bind _box (Variables|Default|GetBox))
  (Rendering|Material|SetVectorParameterValue "/Game/EasySnow/System/MP_WF_WorldData.MP_WF_WorldData" "Location" (Math|Conversions|ToLinearColor(Vector) (Transformation|GetWorldLocation _box)) :!class /Script/Engine.KismetMaterialLibrary)
  (Rendering|Material|SetVectorParameterValue "/Game/EasySnow/System/MP_WF_WorldData.MP_WF_WorldData" "Scale" (Math|Conversions|ToLinearColor(Vector) (Transformation|GetWorldScale _box)) :!class /Script/Engine.KismetMaterialLibrary)
  (Rendering|Material|SetScalarParameterValue "/Game/EasySnow/System/MP_WF_WorldData.MP_WF_WorldData" "Custom Snow Mask Edge Falloff" (Variables|Default|GetcustomSnowMaskEdgeFalloff) :!class /Script/Engine.KismetMaterialLibrary)
  (Rendering|Material|SetScalarParameterValue "/Game/EasySnow/System/MP_WF_WorldData.MP_WF_WorldData" "Custom Snow Mask Breakup Tiling" (Variables|Default|GetcustomSnowMaskBreakupTiling) :!class /Script/Engine.KismetMaterialLibrary)
  (Rendering|Material|SetScalarParameterValue "/Game/EasySnow/System/MP_WF_WorldData.MP_WF_WorldData" "Custom Snow Mask Breakup Contrast" (Variables|Default|GetcustomSnowMaskBreakupContrast) :!class /Script/Engine.KismetMaterialLibrary))